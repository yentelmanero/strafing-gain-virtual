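; BP_Corridor builds a straight two-walled corridor along the X axis between the starting cross and the finish line.
; On BeginPlay it finds BP_StartingCross, then centres WallLeft and WallRight between it and FinishLineReference, separated on Y by Distance.
; Each wall is scaled to the start-to-finish length and Height, assuming a 100-unit mesh, and rolled 90 degrees in opposite directions to stand upright.
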(event `self.ReceiveBeginPlay`
  (bind _height (`self.Height`))
  (bind _returnvalue (/ (`self.Distance`) 2.0))
  (bind _returnvalue_2 (/ _height 2.0))
  (bind _x (.x (`self.K2_GetActorLocation` (`self.StartingCrossReference`))))
  (bind _y (.y (`self.K2_GetActorLocation` (`self.StartingCrossReference`))))
  (bind _returnvalue_3 (- (.x (`self.K2_GetActorLocation` (`self.FinishLineReference`))) _x))
  (bind _returnvalue_4 (`KismetMathLibrary.MakeVector` (/ _returnvalue_3 100.0) (/ _height 100.0) 1.0))
  (bind _returnvalue_5 (+ _x (/ _returnvalue_3 2.0)))
  (bind _returnvalue_6 (`GameplayStatics.GetActorOfClass` "/Game/StrafingGain/BP_StartingCross.BP_StartingCross_C"))
  (set `self.StartingCrossReference` _returnvalue_6)
  (`SceneComponent.K2_SetWorldLocation` (`self.WallLeft`) (`KismetMathLibrary.MakeVector` _returnvalue_5 (- _y _returnvalue) _returnvalue_2) false false)
  (`SceneComponent.K2_SetWorldLocation` (`self.WallRight`) (`KismetMathLibrary.MakeVector` _returnvalue_5 (+ _y _returnvalue) _returnvalue_2) false false)
  (`SceneComponent.SetWorldScale3D` (`self.WallLeft`) _returnvalue_4)
  (`SceneComponent.SetWorldScale3D` (`self.WallRight`) _returnvalue_4)
  (`SceneComponent.K2_SetWorldRotation` (`self.WallLeft`) (`KismetMathLibrary.MakeRotator` 90.0) false false)
  (`SceneComponent.K2_SetWorldRotation` (`self.WallRight`) (`KismetMathLibrary.MakeRotator` -90.0) false false))

(fn `UserConstructionScript`)