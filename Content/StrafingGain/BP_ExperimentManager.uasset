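; Runs a VR strafing-gain experiment, sequencing trials for one participant and section and recording the results.
; After a starting-cross countdown, it draws a random gain without replacement for the pawn and enables WIP, steering or automatic movement.
; A registered 2AFC display stops movement and collects left/right answers, with a periodic FMS rating.
; Per-tick head positions save to CSV each trial; responses and ratings save when the section completes.
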(event `LogPosition`
  (bind _pawnreference (`self.PawnReference`))
  (bind _camera (`/Game/StrafingGain/BP_VRPawn_Strafing.Camera` _pawnreference))
  (bind _returnvalue (`SceneComponent.K2_GetComponentLocation` _camera))
  (`KismetArrayLibrary.Array_Add` (`self.PositionLog`) (`KismetStringLibrary.Concat_StrStr` (`self.ParticipantID`) ";" (`KismetStringLibrary.Conv_Int64ToString` (`KismetSystemLibrary.GetFrameCount`)) ";" (`KismetStringLibrary.Conv_DoubleToString` (- (`KismetSystemLibrary.GetGameTimeInSeconds`) (`self.TrialStartTime`))) ";" (`KismetStringLibrary.Conv_DoubleToString` (.x (- _returnvalue (`self.K2_GetActorLocation` _pawnreference)))) ";" (`KismetStringLibrary.Conv_DoubleToString` (.y (- _returnvalue (`self.K2_GetActorLocation` _pawnreference)))) ";" (`KismetStringLibrary.Conv_DoubleToString` (.z (- _returnvalue (`self.K2_GetActorLocation` _pawnreference)))) ";" (`KismetStringLibrary.Conv_DoubleToString` (.x _returnvalue)) ";" (`KismetStringLibrary.Conv_DoubleToString` (.y _returnvalue)) ";" (`KismetStringLibrary.Conv_DoubleToString` (.z _returnvalue)) ";" (`KismetStringLibrary.Conv_DoubleToString` (.roll (`SceneComponent.K2_GetComponentRotation` _camera))) ";" (`KismetStringLibrary.Conv_DoubleToString` (.pitch (`SceneComponent.K2_GetComponentRotation` _camera))) ";" (`KismetStringLibrary.Conv_DoubleToString` (.yaw (`SceneComponent.K2_GetComponentRotation` _camera))))))

(event `StartCountdown`
  (bind _returnvalue (`GameplayStatics.GetActorOfClass` "/Game/StrafingGain/BP_StartingCross.BP_StartingCross_C"))
  (if (`KismetArrayLibrary.Array_Contains` (`PrimitiveComponent.GetOverlappingActors` (`/Game/StrafingGain/BP_StartingCross.Capsule` _returnvalue) null) (`self.PawnReference`))
    (bind _returnvalue_2 (`GameplayStatics.GetActorOfClass` "/Game/StrafingGain/BP_StartTrialText.BP_StartTrialText_C"))
    (bind _aswbp_start_trial_text (cast `/Game/StrafingGain/UI/WBP_StartTrialText` (`WidgetComponent.GetWidget` (`/Game/StrafingGain/BP_StartTrialText.Widget` _returnvalue_2))))
    (add `/Game/StrafingGain/UI/WBP_StartTrialText.CountdownFinished` _aswbp_start_trial_text (delegate `CountdownDone`))
    (`/Game/StrafingGain/UI/WBP_StartTrialText.CountdownTick` _aswbp_start_trial_text)
    (else
      (bind _returnvalue_3 (`GameplayStatics.GetActorOfClass` "/Game/StrafingGain/BP_StartTrialText.BP_StartTrialText_C"))
      (bind _aswbp_start_trial_text_2 (cast `/Game/StrafingGain/UI/WBP_StartTrialText` (`WidgetComponent.GetWidget` (`/Game/StrafingGain/BP_StartTrialText.Widget` _returnvalue_3))))
      (`/Game/StrafingGain/UI/WBP_StartTrialText.ShowErrorText` _aswbp_start_trial_text_2))))

(event `CountdownDone`
  (`self.SetMovementEnabled` true)
  (`SceneComponent.SetVisibility` (`Actor.RootComponent` (stale `StartCountdown` _returnvalue)) false true)
  (`self.PickNextTrial`)
  (`/Game/StrafingGain/BP_FinishLine.ShowActiveElement` (`self.FinishLine`)))

(event `self.ReceiveTick`
  (params (DeltaSeconds :type "Float (single-precision)"))
  (if (`self.LoggingEnabled`)
    (`self.LogPosition`)))

(event `self.ReceiveBeginPlay`
  (bind _finishline (`self.FinishLine`))
  (bind _returnvalue (`GameplayStatics.GetActorOfClass` "/Game/StrafingGain/BP_VRPawn_Strafing.BP_VRPawn_Strafing_C"))
  (set `self.PawnReference` _returnvalue)
  (set `self.RemainingGains` (`self.GainValues`))
  (bind _returnvalue_2 (`GameplayStatics.GetActorOfClass` "/Game/StrafingGain/BP_FinishLine.BP_FinishLine_C"))
  (set `self.FinishLine` _returnvalue_2)
  (bind _returnvalue_3 (`GameplayStatics.GetActorOfClass` "/Game/StrafingGain/BP_Corridor.BP_Corridor_C"))
  (if (`KismetSystemLibrary.IsValid` _returnvalue_3)
    (set `self.Corridor` _returnvalue_3))
  (set `self.TrialCount` (* (`self.TotalTrials`) (- (`self.Section`) 1)))
  (set `self.TotalTrials` (* (`self.TotalTrials`) (`self.Section`)))
  (if (`/Game/StrafingGain/BP_FinishLine.UseSphere` _finishline)
    (`self.K2_SetActorLocation` _finishline (`KismetMathLibrary.MakeVector` (.x (`self.K2_GetActorLocation` _finishline)) (.y (`self.K2_GetActorLocation` _finishline)) (- (`self.ParticipantHeight`) 30.0)) false false)))

(event `RegisterDisplay`
  (params (Display :type "/Game/StrafingGain/BP_2AFC_Display Object Reference"))
  (bind _output_get (set `self.Current2AFCDisplay` Display))
  (bind _aswbp_2afc (cast `/Game/StrafingGain/UI/WBP_2AFC` (`WidgetComponent.GetWidget` (`/Game/StrafingGain/BP_2AFC_Display.Widget` _output_get))))
  (add `/Game/StrafingGain/UI/WBP_2AFC.OnAnswerGiven` _aswbp_2afc (delegate `OnAnswerReceived`))
  (`self.SetMovementEnabled` false))

(event `OnAnswerReceived`
  (params (MovedLeft :type Boolean))
  (`KismetSystemLibrary.PrintString` "OnAnswerReceived triggered" false)
  (`self.Destroy2AFCDisplay`)
  (if (== (mod (`self.TrialCountForSection`) (`self.FMSFrequency`)) 0)
    (`self.DoFMSScale` MovedLeft)
    (else
      (`self.ProcessResponse` MovedLeft))))

(event `ProcessResponse`
  (params (MovedLeft :type Boolean))
  (bind _responses (`self.Responses`))
  (bind _returnvalue (`KismetStringLibrary.Concat_StrStr` (`self.ParticipantID`) ";" (`|GetEnumeratorNameAsString` (`self.MovementType`)) ";" (`KismetStringLibrary.Conv_IntToString` (`self.TrialCount`)) ";" (`KismetStringLibrary.Conv_DoubleToString` (`self.CurrentGain`)) ";"))
  (if MovedLeft
    (`KismetArrayLibrary.Array_Add` _responses (`KismetStringLibrary.Concat_StrStr` _returnvalue "0"))
    (else
      (`KismetArrayLibrary.Array_Add` _responses (`KismetStringLibrary.Concat_StrStr` _returnvalue "1"))))
  (`self.EndTrial`))

(event `DoFMSScale`
  (params (MovedLeft :type Boolean))
  (bind _location (`/Game/StrafingGain/BP_FinishLine.GetDisplaySpawnLocation` (`self.FinishLine`) (`self.PawnReference`)))
  (bind _returnvalue (`|SpawnActorFromClass` "/Game/StrafingGain/BP_FMS_Display.BP_FMS_Display_C" _location "Undefined" "MultiplyWithRoot" null null))
  (bind _aswbp_fms (cast `/Game/StrafingGain/UI/WBP_FMS` (`WidgetComponent.GetWidget` (`/Game/StrafingGain/BP_FMS_Display.Widget` _returnvalue))))
  (add `/Game/StrafingGain/UI/WBP_FMS.OnFMSSubmitted` _aswbp_fms (delegate `OnFMSResponseReceived`)))

(event `OnFMSResponseReceived`
  (params (FMSValue :type Integer))
  (`KismetArrayLibrary.Array_Add` (`self.FMSValues`) (`KismetStringLibrary.Concat_StrStr` (`self.ParticipantID`) ";" (`|GetEnumeratorNameAsString` (`self.MovementType`)) ";" (`KismetStringLibrary.Conv_IntToString` (/ (`self.TrialCountForSection`) (`self.FMSFrequency`))) ";" (`KismetStringLibrary.Conv_IntToString` FMSValue)))
  (`self.K2_DestroyActor` (stale `DoFMSScale` _returnvalue))
  (`self.ProcessResponse` (stale `DoFMSScale` MovedLeft)))

(event `PickNextTrial`
  (bind _remaininggains (`self.RemainingGains`))
  (bind _returnvalue (`KismetArrayLibrary.Array_Length` (`self.RemainingGains`)))
  (if (== _returnvalue 0)
    (set `self.RemainingGains` (`self.GainValues`)))
  (bind _output_get (set `self.RandomizedIndex` (`KismetMathLibrary.RandomInteger` _returnvalue)))
  (bind _output_get_2 (set `self.CurrentGain` (`|GetArrayItem` _remaininggains _output_get)))
  (`KismetArrayLibrary.Array_Remove` _remaininggains _output_get)
  (bind _output_get_3 (set `/Game/StrafingGain/BP_StrafingGainComponent.CurrentTrialGain` _output_get_2 (`/Game/StrafingGain/BP_VRPawn_Strafing.BP_StrafingGainComponent` (`self.PawnReference`))))
  (set `self.TrialCount` (+ (`self.TrialCount`) 1))
  (set `self.TrialCountForSection` (+ (`self.TrialCountForSection`) 1))
  (`KismetSystemLibrary.PrintString` (`KismetStringLibrary.Concat_StrStr` "Gain for this trial: " (`KismetStringLibrary.Conv_DoubleToString` _output_get_3)) false)
  (set `self.TrialStartTime` (`KismetSystemLibrary.GetGameTimeInSeconds`)))

(event `EndTrial`
  (if (>= (`self.TrialCount`) (`self.TotalTrials`))
    (`KismetSystemLibrary.PrintString` "Completed" false)
    (`self.SavePositionsForTrial`)
    (`self.SaveDataToFile`)
    (bind _location (`/Game/StrafingGain/BP_FinishLine.GetDisplaySpawnLocation` (`self.FinishLine`) (`self.PawnReference`)))
    (`|SpawnActorFromClass` "/Game/StrafingGain/BP_CompleteText.BP_CompleteText_C" _location "Undefined" "MultiplyWithRoot" null null)
    (else
      (`self.ResetTrial`)
      (`self.SavePositionsForTrial`))))

(event `Destroy2AFCDisplay`
  (bind _current2afcdisplay (`self.Current2AFCDisplay`))
  (if (`KismetSystemLibrary.IsValid` _current2afcdisplay)
    (`self.K2_DestroyActor` _current2afcdisplay)))

(event `Recalibrate`
  (bind _corridor (`self.Corridor`))
  (bind _returnvalue (`|SpawnActorFromClass` "/Game/StrafingGain/BP_RecalibrationArrow.BP_RecalibrationArrow_C" (`KismetMathLibrary.Conv_VectorToTransform` (`KismetMathLibrary.MakeVector` (.x (`self.K2_GetActorLocation` (`self.PawnReference`))) (.y (`self.K2_GetActorLocation` (`self.PawnReference`))) 50.0)) "Undefined" "MultiplyWithRoot" null null))
  (add `/Game/StrafingGain/BP_RecalibrationArrow.OnArrowHit` _returnvalue (delegate `ResetTrial`))
  (`/Game/StrafingGain/BP_FinishLine.HideActiveElement` (`self.FinishLine`))
  (if (`KismetSystemLibrary.IsValid` _corridor)
    (`self.SetActorHiddenInGame` _corridor true)))

(event `ResetTrial`
  (bind _corridor (`self.Corridor`))
  (`self.ResetPawnCameraPosition`)
  (`self.Destroy2AFCDisplay`)
  (`/Game/StrafingGain/BP_FinishLine.ShowActiveElement` (`self.FinishLine`))
  (bind _returnvalue (`GameplayStatics.GetActorOfClass` "/Game/StrafingGain/BP_StartTrialText.BP_StartTrialText_C"))
  (bind _aswbp_start_trial_text (cast `/Game/StrafingGain/UI/WBP_StartTrialText` (`WidgetComponent.GetWidget` (`/Game/StrafingGain/BP_StartTrialText.Widget` _returnvalue))))
  (`/Game/StrafingGain/UI/WBP_StartTrialText.ResetTrialText` _aswbp_start_trial_text)
  (bind _returnvalue_2 (`GameplayStatics.GetActorOfClass` "/Game/StrafingGain/BP_StartingCross.BP_StartingCross_C"))
  (`SceneComponent.SetVisibility` (`Actor.RootComponent` _returnvalue_2) true true)
  (if (`KismetSystemLibrary.IsValid` _corridor)
    (`self.SetActorHiddenInGame` _corridor false)))

(event `ResetPawnCameraPosition`
  (bind _pawnreference (`self.PawnReference`))
  (bind _returnvalue (`GameplayStatics.GetActorOfClass` "/Script/Engine.PlayerStart"))
  (bind _returnvalue_2 (`self.K2_GetActorLocation` _returnvalue))
  (`self.K2_SetActorLocation` _pawnreference (`KismetMathLibrary.MakeVector` (.x (- _returnvalue_2 (- (`SceneComponent.K2_GetComponentLocation` (`/Game/StrafingGain/BP_VRPawn_Strafing.Camera` _pawnreference)) (`self.K2_GetActorLocation` _pawnreference)))) (.y (- _returnvalue_2 (- (`SceneComponent.K2_GetComponentLocation` (`/Game/StrafingGain/BP_VRPawn_Strafing.Camera` _pawnreference)) (`self.K2_GetActorLocation` _pawnreference)))) (.z _returnvalue_2)) false false))

(event `SetMovementEnabled`
  (params (Enabled :type Boolean))
  (bind _pawnreference (`self.PawnReference`))
  (set `self.LoggingEnabled` Enabled)
  (set `self.TimeSinceLastLog` 0.0)
  (switch `/Game/StrafingGain/ELocomotionMode` (`self.MovementType`)
    (:`NewEnumerator0`
      (set `/Game/StrafingGain/BP_StrafingGainComponent.WIP_Enabled` Enabled (`/Game/StrafingGain/BP_VRPawn_Strafing.BP_StrafingGainComponent` _pawnreference)))
    (:`NewEnumerator1`
      (set `/Game/StrafingGain/BP_VRPawn_Strafing.SteeringEnabled` Enabled _pawnreference))
    (:`NewEnumerator2`
      (set `/Game/StrafingGain/BP_VRPawn_Strafing.AutoMovement` Enabled _pawnreference))))

(event `SaveDataToFile`
  (bind _prefix (`self.GetFilenamePrefix`))
  (`FileSDKBPLibrary.WriteStringToFile` (`KismetStringLibrary.Concat_StrStr` _prefix "responses_" (`KismetStringLibrary.Conv_IntToString` (`self.Section`)) ".csv") (`KismetStringLibrary.JoinStringArray` (`self.Responses`) " \n"))
  (`FileSDKBPLibrary.WriteStringToFile` (`KismetStringLibrary.Concat_StrStr` _prefix "fms_" (`KismetStringLibrary.Conv_IntToString` (`self.Section`)) ".csv") (`KismetStringLibrary.JoinStringArray` (`self.FMSValues`) " \n")))

(event `SavePositionsForTrial`
  (bind _prefix (`self.GetFilenamePrefix`))
  (`FileSDKBPLibrary.WriteStringToFile` (`KismetStringLibrary.Concat_StrStr` _prefix "position_log_" (`KismetStringLibrary.Conv_IntToString` (`self.TrialCount`)) ".csv") (`KismetStringLibrary.JoinStringArray` (`self.PositionLog`) " \n"))
  (set `self.PositionLog` (`|MakeArray` "UserID;FrameID;Time;PosXReal;PosYReal;PosZReal;PosXVirtual;PosYVirtual;PosZVirtual;Pitch;Yaw;Roll")))

(fn `GetFilenamePrefix`
  (returns (Prefix :type String))
  (return (`KismetStringLibrary.Concat_StrStr` (`KismetSystemLibrary.GetProjectSavedDirectory`) (`self.ParticipantID`) "_")))

(fn `UserConstructionScript`)