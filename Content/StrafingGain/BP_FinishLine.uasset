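; BP_FinishLine is the finish marker in a VR strafing experiment, shown as either a line or a sphere.
; When the strafing VR pawn overlaps it, it spawns a 2AFC display ahead at a camera-based height, registers it with the experiment manager and hides itself.
; Both variants use the line's collision, toggled with actor visibility.
; An optional moving sphere tracks the pawn's X position with an offset each tick.
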(event Custom|ToggleHidden
  (bind _output_get (Variables|Default|SetIsHidden (not (Variables|Default|GetIsHidden))))
  (if _output_get
    (CallFunction|ShowActiveElement)
    (else
      (CallFunction|HideActiveElement))))

(event Custom|HideActiveElement
  (Rendering|SetActorHiddenInGame true)
  (Collision|SetCollisionEnabled (Variables|Default|GetActiveCollision) (Utilities|Enum|LiteralenumECollisionEnabled "NoCollision")))

(event Custom|ShowActiveElement
  (Rendering|SetActorHiddenInGame false)
  (Collision|SetCollisionEnabled (Variables|Default|GetActiveCollision) (Utilities|Enum|LiteralenumECollisionEnabled "QueryAndPhysics")))

(event EventBeginPlay
  (bind _sphere (Variables|Default|GetSphere))
  (bind _line (Variables|Default|GetLine))
  (bind _returnvalue (Actor|GetActorOfClass "/Game/StrafingGain/BP_VRPawn_Strafing.BP_VRPawn_Strafing_C"))
  (Variables|Default|SetPawnReference _returnvalue)
  (if (Variables|Default|GetUseSphere)
    (Variables|Default|SetActiveCollision (Variables|Default|GetLineCollision))
    (Variables|Default|SetActiveElement (Variables|Default|GetSphere))
    (Development|SetHiddeninGame _line true true)
    (Collision|SetCollisionEnabled _line "NoCollision")
    (else
      (Variables|Default|SetActiveCollision (Variables|Default|GetLineCollision))
      (Variables|Default|SetActiveElement (Variables|Default|GetLine))
      (if (Variables|Default|GetMovingSphere)
        _
        (else
          (Development|SetHiddeninGame _sphere true false)))
      (Collision|SetCollisionEnabled _sphere "NoCollision"))))

(event Collision|EventActorBeginOverlap
  (params (OtherActor :type Actor%20Object%20Reference))
  (bind _asbp_vrpawn_strafing (Utilities|Casting|CastToBP_VRPawn_Strafing OtherActor)
    (:then
      (if (stale _bsuccess)
        (Development|PrintString "\"Overlap is VRPawn\"" false)
        (bind _location (CallFunction|GetDisplaySpawnLocation _asbp_vrpawn_strafing))
        (bind _returnvalue (Game|SpawnActorfromClass "/Game/StrafingGain/BP_2AFC_Display.BP_2AFC_Display_C" _location "Undefined" "MultiplyWithRoot" 0 0))
        (bind _returnvalue_2 (Actor|GetActorOfClass "/Game/StrafingGain/BP_ExperimentManager.BP_ExperimentManager_C"))
        (Default|RegisterDisplay _returnvalue_2 _returnvalue)
        (CallFunction|HideActiveElement)
        (else
          (Development|PrintString "\"Overlap not VRPawn\"" false :!label _label))))
    (:CastFailed
      (goto _label))))

(event EventTick
  (params (DeltaSeconds :type Float%20%28single-precision%29))
  (bind _returnvalue (Transformation|GetActorLocation))
  (bind (_x _y _z) (Math|Vector|BreakVector _returnvalue))
  (if (and (Variables|Default|GetMovingSphere) (not (Variables|Default|GetIsHidden)))
    (Transformation|SetRelativeLocation (Variables|Default|GetSphere) (Math|Vector|MakeVector (- (.X (Math|Vector|BreakVector (Transformation|GetActorLocation (Variables|Default|GetPawnReference)))) (Variables|Default|GetPawnOffset)) _y _z) false false)))

(fn ConstructionScript)

(fn GetDisplaySpawnLocation
  (params (Pawn :type BP%20VR%20Pawn%20Strafing%20Object%20Reference))
  (bind _returnvalue (Transformation|GetActorLocation))
  (return (Math|Conversions|ToTransform(Vector) (+ _returnvalue (* (Transformation|GetActorForwardVector) 1.5e+02) (Math|Vector|MakeVector 0.0 0.0 (Utilities|Operators|Subtract (.Z (Math|Vector|BreakVector (Transformation|GetWorldLocation (Variables|/Game/StrafingGain/BP_VRPawn_Strafing.BP_VRPawn_Strafing_C|GetCamera Pawn)))) (.Z (Math|Vector|BreakVector _returnvalue)) 5e+01))))))