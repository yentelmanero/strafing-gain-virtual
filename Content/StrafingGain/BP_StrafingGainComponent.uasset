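; Pawn component for VR walking-in-place locomotion with a strafing gain, an angle that skews each virtual step sideways.
; Tick compares HMD height between frames and fires a step on threshold crossings in both upward and downward directions.
; Each step moves the pawn along the HMD's forward plus right vector scaled by the gain's tangent, with Z zeroed.
; It also accumulates distance and lateral offset, prints movement, and optionally draws a debug arrow.
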(event `self.ReceiveBeginPlay`
  (bind _aspawn (cast `Pawn` (`self.GetOwner`)))
  (set `self.OwnerPawn` _aspawn))

(event `self.ReceiveTick`
  (params (DeltaSeconds :type "Float (single-precision)"))
  (bind _wip_issteppingup (`self.WIP_IsSteppingUp`))
  (bind _hmddata (`HeadMountedDisplayFunctionLibrary.GetHMDData` (`self.OwnerPawn`)))
  (bind _z (.z (`.Position` (break `XRHMDData` _hmddata))))
  (bind _output_get (set `self.WIP_HeightDelta` (- _z (`self.WIP_LastHMDHeight`))))
  (set `self.WIP_LastHMDHeight` _z)
  (`|ExecutionSequence`
    (:`then_0`
      (if (and (> _output_get (`self.WIP_PeakThreshold`)) (not _wip_issteppingup))
        (set `self.WIP_IsSteppingUp` true)
        (`self.StepDetected` :!label _label)))
    (:`then_1`
      (if (and (< _output_get (`self.WIP_ValleyThreshold`)) _wip_issteppingup)
        (set `self.WIP_IsSteppingUp` false)
        (goto _label)))))

(event `StepDetected`
  (bind _wip_stepvirtualdistance (`self.WIP_StepVirtualDistance`))
  (bind _ownerpawn (`self.OwnerPawn`))
  (bind _returnvalue (`Actor.K2_GetActorLocation` _ownerpawn))
  (bind _returnvalue_2 (* _wip_stepvirtualdistance (`KismetMathLibrary.DegTan` (`self.CurrentTrialGain`))))
  (set `self.TotalVirtualDistanceTravelled` (+ (`self.TotalVirtualDistanceTravelled`) _wip_stepvirtualdistance))
  (set `self.TotalPhysicalLateralOffset` (+ (`self.TotalPhysicalLateralOffset`) _returnvalue_2))
  (bind _returnvalue_3 (`KismetMathLibrary.Quat_Rotator` (`.Rotation` (break `XRHMDData` (stale `self.ReceiveTick` _hmddata)))))
  (bind _returnvalue_4 (+ (* (`KismetMathLibrary.GetForwardVector` _returnvalue_3) _wip_stepvirtualdistance) (* (`KismetMathLibrary.GetRightVector` _returnvalue_3) _returnvalue_2)))
  (bind _output_get (set `self.StrafingOffset_ThisTick` (`KismetMathLibrary.MakeVector` (.x _returnvalue_4) (.y _returnvalue_4))))
  (`KismetSystemLibrary.PrintString` (`KismetStringLibrary.Concat_StrStr` " Current Gain: " (`KismetStringLibrary.Conv_DoubleToString` (`self.CurrentTrialGain`)) " Movement this tick: " (`KismetStringLibrary.Conv_VectorToString` _returnvalue_4)))
  (`Actor.K2_AddActorWorldOffset` _ownerpawn _output_get false false)
  (if (`self.DebugEnabled`)
    (`KismetSystemLibrary.DrawDebugArrow` _returnvalue (* (+ _returnvalue _output_get) 50.0) 5.0 (struct :`R` 0.421875 :`B` 0.067284 :`A` 1.0) 0.1 3.0)))