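; BP_TriggerSphere is a trigger actor in a VR strafing experiment that brings up a two-alternative forced choice (2AFC) display.
; When BP_VRPawn_Strafing overlaps it, it spawns BP_2AFC_Display along its forward vector, registers it with the first BP_ExperimentManager found and hides itself.
; Show and hide events switch visibility and collision together.
; ToggleHidden flips IsHidden, showing the sphere when the new value is true.
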(event Custom|ToggleHidden
  (bind _output_get (Variables|Default|SetIsHidden (not (Variables|Default|GetIsHidden))))
  (if _output_get
    (CallFunction|ShowSphere)
    (else
      (CallFunction|HideSphere))))

(event Custom|HideSphere
  (Rendering|SetActorHiddenInGame true)
  (Collision|SetCollisionEnabled (Variables|Default|GetSphere) (Utilities|Enum|LiteralenumECollisionEnabled "NoCollision")))

(event Custom|ShowSphere
  (Rendering|SetActorHiddenInGame false)
  (Collision|SetCollisionEnabled (Variables|Default|GetSphere) (Utilities|Enum|LiteralenumECollisionEnabled "QueryAndPhysics")))

(event EventBeginPlay)

(event Collision|EventActorBeginOverlap
  (params (OtherActor :type Actor%20Object%20Reference))
  (Utilities|Casting|CastToBP_VRPawn_Strafing OtherActor
    (:then
      (if (stale _bsuccess)
        (Development|PrintString "\"Overlap is VRPawn\"")
        (bind _returnvalue (Game|SpawnActorfromClass "/Game/StrafingGain/BP_2AFC_Display.BP_2AFC_Display_C" (Math|Conversions|ToTransform(Vector) (+ (Transformation|GetActorLocation) (* (Transformation|GetActorForwardVector) 1e+02))) "Undefined" "MultiplyWithRoot" 0 0))
        (bind _outactors (Actor|GetAllActorsOfClass "/Game/StrafingGain/BP_ExperimentManager.BP_ExperimentManager_C"))
        (Default|RegisterDisplay (Utilities|Array|Get(acopy) _outactors) _returnvalue)
        (CallFunction|HideSphere)
        (else
          (Development|PrintString "\"Overlap not VRPawn\"" :!label _label))))
    (:CastFailed
      (goto _label))))

(event EventTick
  (params (DeltaSeconds :type Float%20%28single-precision%29)))

(fn ConstructionScript)